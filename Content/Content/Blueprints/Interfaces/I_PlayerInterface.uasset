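; Blueprint interface for the player character, exposing weapon-handling and animation state to other Blueprints such as an animation Blueprint.
; Getters return the left-hand socket transform and IK stop flag, aim state and alpha, hand sway inputs, wall distance, lean directions and an animation state enum.
; One additional function, IF_AddItemToInventory, passes an item and its pickup to the implementer's inventory.
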(fn IFGetLeftHandSocketTransform
  (return ""))

(fn IFGetHandSwayFloats
  (return 0.0 0.0 0.0))

(fn IFGetItsAim
  (return false))

(fn IFGetStopLeftHandIK
  (return false))

(fn IFGetWallDistance
  (return 0.0))

(fn IFAddItemtoInventory
  (params (Item :type BC%20Dynamic%20Inventory%20Item%20Structure) (PickUp :type Actor%20Object%20Reference)))

(fn IFAnimState
  (return "NewEnumerator0"))

(fn IFGetAimAlpha
  (return 0.0))

(fn IFGetLeanBooleans
  (return false false))