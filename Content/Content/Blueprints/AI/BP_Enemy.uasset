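; BP_Enemy is an AI-controlled enemy with a health pool that reacts to damage and dies.
; Each AnyDamage event subtracts the damage from Health and plays a hit reaction montage while Health stays above zero.
; At zero or below, the mesh switches to physics simulation, the AI controller's brain logic stops, and the actor is destroyed after a short delay.
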(event Game|Damage|EventAnyDamage
  (params (Damage :type Float%20%28single-precision%29) (DamageType :type Damage%20Type%20Object%20Reference) (InstigatedBy :type Controller%20Object%20Reference) (DamageCauser :type Actor%20Object%20Reference))
  ;[1 1 1] Take Damage
  (bind _output_get (Variables|Default|SetHealth (Math|Float|Truncate (- (Variables|Default|GetHealth) Damage))))
  (if (<= _output_get 0)
    (Physics|SetSimulatePhysics (Variables|Character|GetMesh) true)
    (bind _asaicontroller (Utilities|Casting|CastToAIController (Pawn|GetController)))
    (AI|Logic|StopLogic (Variables|/Script/AIModule.AIController|GetBrainComponent _asaicontroller) "")
    (Utilities|FlowControl|Delay 5.0)
    (Actor|DestroyActor)
    (else
      (Animation|Montage|PlayMontage (Variables|Character|GetMesh) "/Game/AnimStarterPack/Hit_React_1_Montage.Hit_React_1_Montage"))))

(fn ConstructionScript)